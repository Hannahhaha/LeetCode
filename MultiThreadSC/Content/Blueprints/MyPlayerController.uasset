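; Player controller for a chat screen with a player list, relaying data between the MainUI widget and MyGameMode.
; On the first list update it creates the widget, shows the mouse cursor and binds the widget's send-message delegate.
; Outgoing messages go to the game mode, while received messages and lists update the widget.
; Name changes from UMG set the Name variable and fire a dispatcher; its OnRep is empty.
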(event `OnRecieveList`
  (params (list :type "Array of String"))
  (set `self.tempList` list)
  (`KismetSystemLibrary.PrintString` "update list")
  (`/Engine/EditorBlueprintResources/StandardMacros.IsValid` (`self.MyMainUI`)
    (:`Is Valid`
      _)
    (:`Is Not Valid`
      (bind _returnvalue (`|CreateWidget` "/Game/UI/MainUI.MainUI_C"))
      (`UserWidget.AddToViewport` _returnvalue 0)
      (set `self.MyMainUI` _returnvalue)
      (set `self.bShowMouseCursor` true)
      (add `/Game/UI/MainUI.SendMessageToServer` (`self.MyMainUI`) (delegate `SendMessageToServer_事件_0`))))
  (`/Game/UI/MainUI.UpdatePlayerList` (`self.MyMainUI`) (`self.tempList`)))

(event `OnReceiveMessage`
  (params (newmessage :type String))
  (`/Game/UI/MainUI.AddNewMessage` (`self.MyMainUI`) newmessage))

(event `SendMessageToServer_事件_0`
  (params (Message :type String))
  (`self.SendMessage` Message))

(event `SendMessage`
  (params (message :type String))
  (bind _asmy_game_mode (cast `/Game/Blueprints/MyGameMode` (`GameplayStatics.GetGameMode`)))
  (`/Game/Blueprints/MyGameMode.ReceiveMessage` _asmy_game_mode message))

(event `ChangeName`
  (params (newName :type String))
  (set `self.name` newName)
  (`self.ChangeNameEventDispatcher` newName))

(fn `OnRep_name`)

(fn `UMGChangeName`
  (params (NewName :type String))
  (`self.ChangeName` NewName))

(fn `UserConstructionScript`)