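; Game mode that tracks connected players, keeps their name lists updated and broadcasts messages to all of them.
; PostLogin adds each MyPlayerController to Clients and binds its destroyed and name-change dispatchers.
; Logins, name changes and controller destruction, which stands in for logout, trigger sending the list of names to every client.
; ReceiveMessage relays a message to every controller in Clients through OnReceiveMessage.
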(event `self.K2_PostLogin`
  (params (NewPlayer :type "PlayerController Object Reference"))
  (bind _asmy_player_controller (cast `/Game/Blueprints/MyPlayerController` NewPlayer))
  (`self.HandlePlayerLogin` _asmy_player_controller)
  (add `self.OnDestroyed` _asmy_player_controller (delegate `OnDestroyed_事件_0`))
  (add `/Game/Blueprints/MyPlayerController.ChangeNameEventDispatcher` _asmy_player_controller (delegate `ChangeNameEventDispatcher_事件_0`)))

(event `ChangeNameEventDispatcher_事件_0`
  (params (name :type String))
  (`self.SendPlayerListToAll`))

(event `OnDestroyed_事件_0` :!signature `self.OnDestroyed`
  (params (DestroyedActor :type "Actor Object Reference"))
  (`self.HandlePlayerLoginOut` (stale `self.K2_PostLogin` _asmy_player_controller)))

(fn `HandlePlayerLogin`
  (params (Player :type "/Game/Blueprints/MyPlayerController Object Reference"))
  (`KismetArrayLibrary.Array_Add` (`self.Clients`) Player)
  (`self.SendPlayerListToAll`))

(fn `HandlePlayerLoginOut`
  (params (player :type "/Game/Blueprints/MyPlayerController Object Reference"))
  (`KismetArrayLibrary.Array_RemoveItem` (`self.Clients`) player)
  (`self.SendPlayerListToAll`))

(fn `ReceiveChangeName`
  (`self.SendPlayerListToAll`))

(fn `ReceiveMessage`
  (params (msg :type String))
  (for _array_element (`self.Clients`)
    (`/Game/Blueprints/MyPlayerController.OnReceiveMessage` _array_element msg)))

(fn `ReturnPlayerListToClient`
  (params (list :type "Array of String") (who :type "/Game/Blueprints/MyPlayerController Object Reference"))
  (`/Game/Blueprints/MyPlayerController.OnRecieveList` who list))

(fn `SendPlayerListToAll`
  (locals (TempList :type "Array of String"))
  (for _array_element (`self.Clients`)
    (`KismetArrayLibrary.Array_Add` (`local.TempList`) (`/Game/Blueprints/MyPlayerController.name` _array_element)))
  (for _array_element_2 (`self.Clients`)
    (`self.ReturnPlayerListToClient` (`local.TempList`) _array_element_2)))

(fn `UserConstructionScript`)